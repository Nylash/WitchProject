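; First-person player character that moves, crouches, and picks up, drags and places objects with a physics handle.
; Camera line traces find interactables and snap points, driving HUD cursor icons and custom-depth outlines.
; Interact grabs items, spawns them from spawners matched by class-name prefix to a data table, or checks receptacles.
; Held items drop onto snap points, while other objects slide along camera forward using look input until released.
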(event EventTick
  (params (DeltaSeconds :type Float%20%28single-precision%29))
  (Utilities|FlowControl|Sequence
    (:then_0
      ;[1 1 1] Set Handle Location
      (if (Variables|Default|GetIssliding)
        ;[1 1 1] Cursor handling
        (bind (_returnvalue _location _actor) (CallFunction|LineTraceInteractableObjects :!label _label))
        (if _returnvalue
          (CallFunction|ChangeCursor true false)
          ;[1 1 1] Outline
          (if (Variables|Default|GetIsholding)
            _
            (else
              (if (== _actor (Variables|Default|GetInteractable))
                _
                (else
                  (CallFunction|DoOutline _actor (Variables|Default|GetInteractable))))
              (Variables|Default|SetInteractable _actor)
              (goto _label_2 Reset)))
          (else
            (CallFunction|ChangeCursor false false)))
        (Utilities|FlowControl|DoOnce false :!label _label_2
          (:Completed
            (CallFunction|EraseOutline)))
        (else
          (Physics|Components|PhysicsHandle|SetTargetLocation (Variables|Default|GetPhysicsHandle) (Transformation|GetWorldLocation (Variables|Default|GetGrab%20Location)))
          (if (Variables|Default|GetIsholding)
            ;[1 1 1] Handling dragable object max distance
            (Utilities|Casting|CastToBasic_Item (Variables|Default|GetGrab%20Actor)
              (:CastFailed
                (if (> (Math|Vector|Distance(Vector) (Transformation|GetWorldLocation (Variables|Default|GetPhysics%20Object)) (Transformation|GetWorldLocation (Variables|Default|GetGrab%20Location))) 2e+03)
                  (CallFunction|Drop)
                  (goto _label))))
            (else
              (goto _label))))))
    (:then_1
      (if (Variables|Default|GetIsholding)
        (bind (_returnvalue_2 _location_2) (CallFunction|LineTraceSnapObjects))
        (if _returnvalue_2
          (CallFunction|ChangeCursor false true)
          (Variables|Default|SetSnapLocation _location_2)
          (else
            (CallFunction|ChangeCursor false false)))))))

(event EventBeginPlay
  ;[1 1 1] Generate HUD
  (bind _returnvalue (UserInterface|CreateWidget "/Game/Assets/UI/HUD.HUD_C" (Game|GetPlayerController 0)))
  (bind _output_get (Variables|Default|SetHUD _returnvalue))
  (UserInterface|Viewport|AddtoViewport _output_get 0)
  (Class|Image|SetOpacity (Variables|/Game/Assets/UI/HUD.HUD_C|GetHand_Image (Variables|Default|GetHUD)) 0.0))

(event Input|ActionEvents|InputActionInteract
  (params (Key :type Key%20Structure))
  ;[1 1 1] Input for PickUp
  (:Pressed
    (if (Variables|Default|GetIsholding)
      (CallFunction|Drop :!label _label)
      (else
        (CallFunction|PickUp))))
  (:Released
    (if (Variables|Default|GetIssliding)
      (goto _label))))

(event Input|ActionEvents|InputActionCrouch
  (params (Key :type Key%20Structure))
  ;[1 1 1] Crouch
  (:Pressed
    (Character|Crouch))
  (:Released
    (Character|UnCrouch)))

(event Input|AxisEvents|InputAxisMoveForward
  (params (AxisValue :type Float%20%28single-precision%29))
  ;[1 1 1] Movement
  (Pawn|Input|AddMovementInput (Math|Vector|GetForwardVector (Pawn|GetControlRotation :!class /Script/Engine.Pawn)) AxisValue false))

(event Input|AxisEvents|InputAxisMoveRight
  (params (AxisValue :type Float%20%28single-precision%29))
  ;[1 1 1] Movement
  (Pawn|Input|AddMovementInput (Math|Vector|GetRightVector (Pawn|GetControlRotation :!class /Script/Engine.Pawn)) AxisValue false))

(event Input|AxisEvents|InputAxisCameraUp
  (params (AxisValue :type Float%20%28single-precision%29))
  ;[1 1 1] Camera
  (if (Variables|Default|GetIssliding)
    (CallFunction|UpdateSlide AxisValue)
    (else
      (Pawn|Input|AddControllerPitchInput AxisValue))))

(event Input|AxisEvents|InputAxisCameraRight
  (params (AxisValue :type Float%20%28single-precision%29))
  ;[1 1 1] Camera
  (if (Variables|Default|GetIssliding)
    (CallFunction|UpdateSlide AxisValue)
    (else
      (Pawn|Input|AddControllerYawInput AxisValue))))

(fn ConstructionScript)

(fn PickUp
  (bind (_returnvalue _location _actor _component) (CallFunction|LineTraceInteractableObjects))
  (if _returnvalue
    (Variables|Default|SetGrab%20Actor _actor)
    (if (Utilities|Enum|Equal(Enum) (Utilities|String|GetSubstring (Utilities|GetClassDisplayName (Utilities|GetClass (Variables|Default|GetGrab%20Actor))) 0 2) "Sp")
      ;[1 1 1] Spawn item thanks to data table reference then grab it
      (bind _returnvalue_2 (Utilities|GetDataTableRow "/Game/Blueprints/SpawnerDataTable.SpawnerDataTable" (Utilities|String|StringToName (Utilities|String|GetSubstring (Utilities|GetClassDisplayName (Utilities|GetClass (Variables|Default|GetGrab%20Actor))) 0 4)))
        (:then
          (bind _asbasic_spawner (Utilities|Casting|CastToBasic_Spawner (Variables|Default|GetGrab%20Actor)))
          (bind (_actor_2 _primitivecomponent) (Default|Spawn _asbasic_spawner (Utilities|Struct|BreakSpawnerStructure _returnvalue_2) (Transformation|GetWorldLocation (Variables|Default|GetGrab%20Location))))
          (bind _output_get (Variables|Default|SetPhysics%20Object _primitivecomponent))
          (Variables|Default|SetGrab%20Actor _actor_2)
          (Class|PhysicsHandleComponent|GrabComponentatLocation (Variables|Default|GetPhysicsHandle) _output_get "None" (Transformation|GetWorldLocation _primitivecomponent))))
      (else
        (Utilities|Casting|CastToBasic_Item (Variables|Default|GetGrab%20Actor)
          (:then
            ;[1 1 1] Handling unique object
            (bind _output_get_2 (Variables|Default|SetPhysics%20Object _component))
            (Class|PhysicsHandleComponent|GrabComponentatLocation (Variables|Default|GetPhysicsHandle) _output_get_2 "None" (Transformation|GetWorldLocation _output_get_2)))
          (:CastFailed
            ;[1 1 1] Handling dragable object
            (bind _output_get_3 (Variables|Default|SetPhysics%20Object _component))
            (Class|PhysicsHandleComponent|GrabComponentatLocation (Variables|Default|GetPhysicsHandle) _output_get_3 "None" _location)
            (Physics|SetSimulatePhysics _output_get_3 true)
            (Variables|Default|SetIssliding true)))))
    (Variables|Default|SetIsholding true)
    (Collision|SetCollisionResponsetoChannel (Variables|Default|GetPhysics%20Object) "ECC_Pawn" "ECR_Ignore")
    (Collision|SetCollisionResponsetoChannel (Variables|Default|GetPhysics%20Object) "ECC_GameTraceChannel1" "ECR_Ignore")
    (CallFunction|ChangeCursor false false)
    (bind _asbasic_item (Utilities|Casting|CastToBasic_Item (Variables|Default|GetGrab%20Actor)))
    (Default|EnabledTaken _asbasic_item)
    (else
      (bind (_returnvalue_3 _location_2 _actor_3) (CallFunction|LineTraceSnapObjects))
      (if _returnvalue_3
        ;[1 1 1] receptacle
        (bind _asreceptacle (Utilities|Casting|CastToReceptacle _actor_3))
        (Default|CheckItem _asreceptacle)))))

(fn Drop
  (bind _physics_object (Variables|Default|GetPhysics%20Object))
  ;[1 1 1] Drop Object function
  (Physics|Components|PhysicsHandle|ReleaseComponent (Variables|Default|GetPhysicsHandle))
  (if (Variables|Default|GetArrowDisplaying)
    ;[1 1 1] Object On Snap
    (bind _asbasic_item (Utilities|Casting|CastToBasic_Item (Variables|Default|GetGrab%20Actor)))
    (Transformation|SetWorldLocation (Variables|/Game/Blueprints/Items/Basic_Item.Basic_Item_C|GetStaticMesh _asbasic_item) (Variables|Default|GetSnapLocation) true false))
  (Variables|Default|SetIsholding false)
  (Collision|SetCollisionResponsetoChannel _physics_object "ECC_Pawn" "ECR_Block")
  (Collision|SetCollisionResponsetoChannel _physics_object "ECC_GameTraceChannel1" "ECR_Block")
  (Class|PrimitiveComponent|SetAllPhysicsLinearVelocity _physics_object "0, 0, 0" false)
  (bind _asbasic_item_2 (Utilities|Casting|CastToBasic_Item (Variables|Default|GetGrab%20Actor))
    (:then
      (Default|EnabledTaken _asbasic_item_2))
    (:CastFailed
      (Physics|SetSimulatePhysics (Variables|Default|GetPhysics%20Object) false)
      (Variables|Default|SetIssliding false))))

(fn ChangeCursor
  (params (DisplayHand :type Boolean) (DisplayArrow :type Boolean))
  (bind _hud (Variables|Default|GetHUD))
  (bind _hud_2 (Variables|Default|GetHUD))
  (bind _hud_3 (Variables|Default|GetHUD))
  (if DisplayArrow
    ;[1 1 1] Display Arrow
    (Class|Image|SetOpacity (Variables|/Game/Assets/UI/HUD.HUD_C|GetHand_Image _hud_3) 0.0)
    (Class|Image|SetOpacity (Variables|/Game/Assets/UI/HUD.HUD_C|GetCursor_Image _hud_3) 0.0)
    (Class|Image|SetOpacity (Variables|/Game/Assets/UI/HUD.HUD_C|GetArrow_Image _hud_3) 1.0)
    (Variables|Default|SetArrowDisplaying true)
    (elif DisplayHand
      ;[1 1 1] Display Hand
      (if (not (Variables|Default|GetIsholding))
        (if (not (Variables|Default|GethandDisplayed))
          (Class|Image|SetOpacity (Variables|/Game/Assets/UI/HUD.HUD_C|GetHand_Image _hud) 1.0)
          (Class|Image|SetOpacity (Variables|/Game/Assets/UI/HUD.HUD_C|GetCursor_Image _hud) 0.0)
          (Class|Image|SetOpacity (Variables|/Game/Assets/UI/HUD.HUD_C|GetArrow_Image _hud) 0.0)
          (Variables|Default|SethandDisplayed true)
          (Variables|Default|SetArrowDisplaying false)))
      (else
        ;[1 1 1] Display Cursor
        (Class|Image|SetOpacity (Variables|/Game/Assets/UI/HUD.HUD_C|GetHand_Image _hud_2) 0.0)
        (Class|Image|SetOpacity (Variables|/Game/Assets/UI/HUD.HUD_C|GetCursor_Image _hud_2) 1.0)
        (Class|Image|SetOpacity (Variables|/Game/Assets/UI/HUD.HUD_C|GetArrow_Image _hud_2) 0.0)
        (Variables|Default|SethandDisplayed false)
        (Variables|Default|SetArrowDisplaying false)))))

(fn LineTraceInteractableObjects
  (bind _camera (Variables|Default|GetCamera))
  (bind _returnvalue (Transformation|GetWorldLocation _camera))
  (bind (_outhit _returnvalue_2) (Collision|LineTraceForObjects _returnvalue (+ _returnvalue (* (Math|Vector|GetForwardVector _camera) (Variables|Default|GetMaxDistancePickUp))) (Utilities|Array|MakeArray "ObjectTypeQuery7") false 0 "None"))
  (return _returnvalue_2 (.Location (Collision|BreakHitResult _outhit)) (.HitActor (Collision|BreakHitResult _outhit)) (.HitComponent (Collision|BreakHitResult _outhit))))

(fn DoOutline
  (params (NewActor :type Actor%20Object%20Reference) (OldActor :type Actor%20Object%20Reference))
  ;[1 1 1] Change custom depth of new actor and reset old actor's one
  (Rendering|SetRenderCustomDepth (Utilities|Array|Get(acopy) (Actor|GetComponentsbyTag NewActor "/Script/Engine.PrimitiveComponent" "Outline")) true)
  (if (!= OldActor 0)
    (Rendering|SetRenderCustomDepth (Utilities|Array|Get(acopy) (Actor|GetComponentsbyTag OldActor "/Script/Engine.PrimitiveComponent" "Outline")) false)))

(fn EraseOutline
  ;[1 1 1] Erase outline if there is no result to line trace
  (if (!= (Variables|Default|GetInteractable) 0)
    (Rendering|SetRenderCustomDepth (Utilities|Array|Get(acopy) (Actor|GetComponentsbyTag (Variables|Default|GetInteractable) "/Script/Engine.PrimitiveComponent" "Outline")) false)
    (Variables|Default|SetInteractable 0)))

(fn UpdateSlide
  (params (SlideForce :type Float%20%28single-precision%29))
  (Physics|Components|PhysicsHandle|SetTargetLocation (Variables|Default|GetPhysicsHandle) (+ (.TargetLocation (Class|PhysicsHandleComponent|GetTargetLocationandRotation (Variables|Default|GetPhysicsHandle))) (* (Math|Vector|GetForwardVector (Variables|Default|GetCamera)) (* SlideForce -1.0)))))

(fn LineTraceSnapObjects
  (bind _camera (Variables|Default|GetCamera))
  (bind _returnvalue (Transformation|GetWorldLocation _camera))
  (bind (_outhit _returnvalue_2) (Collision|LineTraceForObjects _returnvalue (+ _returnvalue (* (Math|Vector|GetForwardVector _camera) (Variables|Default|GetMaxDistancePickUp))) (Utilities|Array|MakeArray "ObjectTypeQuery8") false (Utilities|Array|MakeArray (Game|Player|GetPlayerPawn 0)) "None"))
  (return _returnvalue_2 (.Location (Collision|BreakHitResult _outhit)) (.HitActor (Collision|BreakHitResult _outhit)) (.HitComponent (Collision|BreakHitResult _outhit))))