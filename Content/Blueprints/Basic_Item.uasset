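; Basic_Item is an item Blueprint with a static mesh that turns to face the player character while its Taken flag is set.
; Each tick it rotates the mesh toward player 0 using a look-at rotation and prints a debug yes or no for the flag.
; The EnabledTaken function toggles Taken.
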(event EventTick
  (params (DeltaSeconds :type Float%20%28single-precision%29))
  (bind _staticmesh (Variables|Default|GetStaticMesh))
  (if (Variables|Default|GetTaken)
    (Development|PrintString "yes")
    (Transformation|SetWorldRotation _staticmesh (Math|Conversions|RotationFromXVector (Math|Rotator|GetRotationXVector (Math|Rotator|FindLookatRotation (Transformation|GetWorldLocation _staticmesh) (Transformation|GetActorLocation (Game|GetPlayerCharacter 0))))) false false)
    (else
      (Development|PrintString "no"))))

(fn ConstructionScript)

(fn EnabledTaken
  (if (Variables|Default|GetTaken)
    (Variables|Default|SetTaken false)
    (else
      (Variables|Default|SetTaken true)))
  (return))