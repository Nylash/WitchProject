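; Crafting receptacle that combines two or three Basic_Items into a recipe result.
; While an actor overlaps it, a 0.1s tick box-traces for untaken items and lists their IDs on the HUD.
; CheckItem pads pairs with a temporary It00 item, then scans RecipesDataBase for an order-independent match.
; A match destroys the inputs and spawns the class from SpawnerRecipeDataTable at the same index; failures show HUD messages.
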(event Collision|EventActorBeginOverlap
  (params (OtherActor :type Actor%20Object%20Reference))
  (Variables|Default|SetplayerIn true))

(event Collision|EventActorEndOverlap
  (params (OtherActor :type Actor%20Object%20Reference))
  (Variables|Default|SetplayerIn false))

(event EventTick
  (params (DeltaSeconds :type Float%20%28single-precision%29))
  (bind _hud (Variables|Default|GetHUD))
  (if (Variables|Default|GetplayerIn)
    (bind (_out_hits _return_value) (CallFunction|MultiBox))
    ;[1 1 1] Verify if ingredients got theirs lines written, else write it only once
    (if _return_value
      (if (not (Math|Boolean|ANDBoolean (== (Utilities|Array|Length _out_hits) 1) (Variables|Default|GetIng1Here) (not (Variables|Default|GetIng2Here))))
        (if (not (Math|Boolean|ANDBoolean (== (Utilities|Array|Length _out_hits) 2) (Variables|Default|GetIng2Here) (not (Variables|Default|GetIng3Here))))
          (if (not (and (== (Utilities|Array|Length _out_hits) 3) (Variables|Default|GetIng3Here)))
            (CallFunction|CleanBoardUpdate)
            (for _array_element _out_hits
              ;[1 1 1] Add a new line from the new ingredient
              (bind _asbasic_item (Utilities|Casting|CastToBasic_Item (.HitActor (Collision|BreakHitResult _array_element))))
              (if (not (Variables|/Game/Blueprints/Items/Basic_Item.Basic_Item_C|GetTaken _asbasic_item))
                (if (Variables|Default|GetIng1Here)
                  (if (Variables|Default|GetIng2Here)
                    (if (not (Variables|Default|GetIng3Here))
                      (Variables|Default|SetIng3Here true)
                      (Rendering|Components|TextRender|SetText (Variables|/Game/Blueprints/HUD.HUD_C|GetIng3 _hud) (Utilities|Text|ToText(String) (Variables|/Game/Blueprints/Items/Basic_Item.Basic_Item_C|GetID _asbasic_item))))
                    (else
                      (Variables|Default|SetIng2Here true)
                      (Rendering|Components|TextRender|SetText (Variables|/Game/Blueprints/HUD.HUD_C|GetIng2 _hud) (Utilities|Text|ToText(String) (Variables|/Game/Blueprints/Items/Basic_Item.Basic_Item_C|GetID _asbasic_item)))))
                  (else
                    (Variables|Default|SetIng1Here true)
                    (Rendering|Components|TextRender|SetText (Variables|/Game/Blueprints/HUD.HUD_C|GetIng1 _hud) (Utilities|Text|ToText(String) (Variables|/Game/Blueprints/Items/Basic_Item.Basic_Item_C|GetID _asbasic_item)))))))))))))

(event EventBeginPlay
  (Actor|Tick|SetActorTickInterval 0.1))

(fn ConstructionScript)

(fn CheckItem
  (bind _objects_in_rec (Variables|Default|GetObjects%20In%20Rec))
  (bind _returnvalue (Utilities|Array|Length _objects_in_rec))
  (Utilities|Array|Clear (Variables|Default|GetObjects%20In%20Rec))
  (bind (_out_hits _return_value) (CallFunction|MultiBox))
  (if _return_value
    (for _array_element _out_hits
      (Utilities|Array|Add (Variables|Default|GetObjects%20In%20Rec) (.HitActor (Collision|BreakHitResult _array_element))))
    (if (== _returnvalue 1)
      (CallFunction|SendMessage "NewEnumerator0")
      (elif (== _returnvalue 2)
        (bind _returnvalue_2 (Game|SpawnActorfromClass "/Game/Blueprints/Items/It00.It00_C" (Math|Conversions|ToTransform(Vector) (Math|Vector|VectorZero)) "AlwaysSpawn" 0 0))
        (Utilities|Array|Add (Variables|Default|GetObjects%20In%20Rec) _returnvalue_2)
        (bind (_recipeexist _recipeindex) (CallFunction|CheckRecipe :!label _label))
        (if _recipeexist
          (CallFunction|SpawnRecipe _recipeindex)
          (else
            ;[1 1 1] Handle bad recipe
            (CallFunction|SendMessage "NewEnumerator3")))
        (if (Utilities|IsValid _returnvalue_2)
          (Actor|DestroyActor _returnvalue_2))
        (elif (== _returnvalue 3)
          (goto _label)
          (else
            (CallFunction|SendMessage "NewEnumerator1")))))))

(fn CheckRecipe
  (LocalVariables|SetFirstIngFound false)
  (LocalVariables|SetSecIngFound false)
  (LocalVariables|SetThrdIngFound false)
  (bind _index (Utilities|FlowControl|ForLoopwithBreak 0 82 :!label _label)
    (:LoopBody
      (bind _returnvalue (Utilities|GetDataTableRow "/Game/Blueprints/RecipesDataBase.RecipesDataBase" (Utilities|String|StringToName (Utilities|String|ToString(Integer) _index)))
        (:then
          (bind _array_element (Utilities|Array|ForEachLoopwithBreak (Variables|Default|GetObjects%20In%20Rec) :!label _label_2)
            (:LoopBody
              (bind _asbasic_item (Utilities|Casting|CastToBasic_Item _array_element))
              (if (Utilities|Array|ContainsItem (Utilities|Array|MakeArray (.Ing1 (Utilities|Struct|BreakRecipeStructure _returnvalue)) (.Ing2 (Utilities|Struct|BreakRecipeStructure _returnvalue)) (.Ing3 (Utilities|Struct|BreakRecipeStructure _returnvalue))) (Variables|/Game/Blueprints/Items/Basic_Item.Basic_Item_C|GetID _asbasic_item))
                (if (LocalVariables|GetFirstIngFound)
                  (if (LocalVariables|GetSecIngFound)
                    (if (not (LocalVariables|GetThrdIngFound))
                      (LocalVariables|SetThrdIngFound true))
                    (else
                      (LocalVariables|SetSecIngFound true)))
                  (else
                    (LocalVariables|SetFirstIngFound true)))
                (else
                  (LocalVariables|SetFirstIngFound false)
                  (LocalVariables|SetSecIngFound false)
                  (LocalVariables|SetThrdIngFound false)
                  (goto _label_2 Break))))
            (:Completed
              (if (LocalVariables|GetThrdIngFound)
                (goto _label Break)))))))
    (:Completed
      (return (LocalVariables|GetThrdIngFound) _index))))

(fn SpawnRecipe
  (params (IndexRecipe :type Integer))
  (bind _returnvalue (Utilities|String|ToString(Integer) IndexRecipe))
  (CallFunction|CleanReceptacle)
  (CallFunction|CleanBoardUpdate)
  (bind _returnvalue_2 (Utilities|GetDataTableRow "/Game/Blueprints/SpawnerRecipeDataTable.SpawnerRecipeDataTable" (Utilities|String|StringToName _returnvalue))
    (:then
      (Game|SpawnActorfromClass (.ClassToSpawn (Utilities|Struct|BreakSpawnerStructure _returnvalue_2)) (Math|Conversions|ToTransform(Vector) (Transformation|GetWorldLocation (Variables|Default|GetSpawnLocation))) "AdjustIfPossibleButAlwaysSpawn" 0 0)
      (if (not (Utilities|IsValidClass (.ClassToSpawn (Utilities|Struct|BreakSpawnerStructure _returnvalue_2))))
        (CallFunction|SendMessage "NewEnumerator2")))
    (:RowNotFound
      ;[1 1 1] Debug
      (Development|PrintString "Une recette non valide a été validé (Spawnrecipe) index de la recette ci dessous")
      (Development|PrintString _returnvalue))))

(fn CleanReceptacle
  (for _array_element (Variables|Default|GetObjects%20In%20Rec)
    (Actor|DestroyActor _array_element)))

(fn SendMessage
  (params (NewParam :type Messages%20Enum :default "NewEnumerator5"))
  (bind _asplayer (Utilities|Casting|CastToPlayer (Game|Player|GetPlayerPawn 0)))
  (if (Variables|/Game/Blueprints/Player.Player_C|GetTextInUse _asplayer)
    (Development|PrintString "Hello")
    (else
      (Rendering|Components|TextRender|SetText (Variables|/Game/Blueprints/HUD.HUD_C|GetMessage (Variables|Default|GetHUD)) (Utilities|Text|ToText(String) (Utilities|String|EnumtoString NewParam)))
      (Variables|/Game/Blueprints/Player.Player_C|SetTextInUse _asplayer true)
      (Variables|/Game/Blueprints/Player.Player_C|SetTextWritten _asplayer true))))

(fn MultiBox
  (bind _spawnlocation (Variables|Default|GetSpawnLocation))
  (bind _returnvalue (Transformation|GetWorldLocation _spawnlocation))
  (bind (_outhits _returnvalue_2) (Class|KismetSystemLibrary|BoxTraceMultiforObjects _returnvalue (+ _returnvalue (* (Math|Vector|GetUpVector _spawnlocation) (Variables|Default|Getreach))) (Math|Conversions|ToVector(Float) (Variables|Default|GetSize)) "0, 0, 0" (Utilities|Array|MakeArray "ObjectTypeQuery7") false 0 "ForDuration" true))
  (for _array_element _outhits
    (bind _asbasic_item (Utilities|Casting|CastToBasic_Item (.HitActor (Collision|BreakHitResult _array_element))))
    (if (Variables|/Game/Blueprints/Items/Basic_Item.Basic_Item_C|GetTaken _asbasic_item)
      (Utilities|Array|RemoveItem _outhits _array_element)))
  (return _outhits _returnvalue_2))

(fn CleanBoardUpdate
  (bind _hud (Variables|Default|GetHUD))
  (Variables|Default|SetIng1Here false)
  (Variables|Default|SetIng2Here false)
  (Variables|Default|SetIng3Here false)
  (Rendering|Components|TextRender|SetText (Variables|/Game/Blueprints/HUD.HUD_C|GetIng1 _hud) "")
  (Rendering|Components|TextRender|SetText (Variables|/Game/Blueprints/HUD.HUD_C|GetIng2 _hud) "")
  (Rendering|Components|TextRender|SetText (Variables|/Game/Blueprints/HUD.HUD_C|GetIng3 _hud) ""))